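; Black hole projectile that destroys physics-simulating actors it hits and removes itself after five seconds.
; On BeginPlay its sphere ignores the instigator while moving and a one-shot timer starts for self-destruction.
; Every Tick calls AddRadialForce on the sphere component itself with a large negative strength and constant falloff.
; The sphere's hit event destroys the other actor only if its root component simulates physics.
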(event OnProjectileStop(MovementComponent)
  (params (ImpactResult :type Hit%20Result%20Structure%20%28by%20ref%29)))

(event OnComponentHit(SphereComponent)
  (params (HitComponent :type Primitive%20Component%20Object%20Reference) (OtherActor :type Actor%20Object%20Reference) (OtherComp :type Primitive%20Component%20Object%20Reference) (NormalImpulse :type Vector :default "0, 0, 0") (Hit :type Hit%20Result%20Structure%20%28by%20ref%29))
  (if (Physics|IsSimulatingPhysics (Variables|/Script/Engine.Actor|GetRootComponent OtherActor) "None")
    (Actor|DestroyActor OtherActor)))

(event Custom|TimerOver
  (Actor|DestroyActor))

(event EventBeginPlay
  (Collision|IgnoreActorwhenMoving (Variables|Default|GetSphereComponent) (Game|GetInstigator) true)
  (Utilities|Time|SetTimerbyEvent (delegate Custom|TimerOver) 5.0))

(event EventTick
  (params (DeltaSeconds :type Float%20%28single-precision%29))
  (Physics|AddRadialForce (Variables|Default|GetSphereComponent) "0, 0, 0" 4e+02 -1e+06 "RIF_Constant" false))

(fn ConstructionScript)